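; BP_Tunnel is an endless-tunnel segment that asks TunnelSpawner for a new segment and destroys itself when the player crosses its trigger, adding score.
; On BeginPlay it randomly keeps an offset health pack and spawns enemies linked to it as Master.
; Tick spins the wall and pack; touching the wall costs health and score, bullets die on it, and the pack heals.
; RandomizeWall picks a hole mesh and roll, but is not called here.
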(event OnComponentBeginOverlap(TriggerZone)
  (params (OverlappedComponent :type Primitive%20Component%20Object%20Reference) (OtherActor :type Actor%20Object%20Reference) (OtherComp :type Primitive%20Component%20Object%20Reference) (OtherBodyIndex :type Integer) (bFromSweep :type Boolean) (SweepResult :type Hit%20Result%20Structure%20%28by%20ref%29))
  (bind _asbp_player (Utilities|Casting|CastToBP_Player OtherActor))
  (Default|SpawnTunnelatSpawnPoint (Variables|Default|GetTunnelSpawner))
  (Actor|DestroyActor)
  (Default|IncreaseScore _asbp_player 1)
  (Default|RenderScore _asbp_player))

(event OnComponentHit(HealthPack)
  (params (HitComponent :type Primitive%20Component%20Object%20Reference) (OtherActor :type Actor%20Object%20Reference) (OtherComp :type Primitive%20Component%20Object%20Reference) (NormalImpulse :type Vector :default "0, 0, 0") (Hit :type Hit%20Result%20Structure%20%28by%20ref%29))
  (bind _asbp_player (Utilities|Casting|CastToBP_Player OtherActor))
  (Default|DecreaseHealth _asbp_player -15)
  (Components|DestroyComponent HitComponent))

(event OnComponentBeginOverlap(WallMesh)
  (params (OverlappedComponent :type Primitive%20Component%20Object%20Reference) (OtherActor :type Actor%20Object%20Reference) (OtherComp :type Primitive%20Component%20Object%20Reference) (OtherBodyIndex :type Integer) (bFromSweep :type Boolean) (SweepResult :type Hit%20Result%20Structure%20%28by%20ref%29))
  (bind _asbp_player (Utilities|Casting|CastToBP_Player OtherActor)
    (:then
      (Default|DecreaseHealth _asbp_player 10)
      (Default|IncreaseScore _asbp_player -1))
    (:CastFailed
      (bind _asbullet (Utilities|Casting|CastToBullet OtherActor))
      (Actor|DestroyActor _asbullet))))

(event EventBeginPlay
  (CallFunction|GenerateHealthPack)
  (CallFunction|GenerateEnemies))

(event EventTick
  (params (DeltaSeconds :type Float%20%28single-precision%29))
  (bind _healthpack (Variables|Default|GetHealthPack))
  (bind _rotatespeed (Variables|Default|GetRotateSpeed))
  (bind _returnvalue (* DeltaSeconds _rotatespeed))
  (Transformation|AddLocalRotation (Variables|Default|GetWallMesh) (Math|Rotator|MakeRotator _returnvalue 0.0 0.0) false false)
  (Utilities|IsValid _healthpack
    (:Is%20Valid
      (Transformation|AddLocalRotation _healthpack (Math|Rotator|MakeRotator _returnvalue _returnvalue _returnvalue) false false))))

(fn ConstructionScript)

(fn RandomizeWall
  (Components|StaticMesh|SetStaticMesh (Variables|Default|GetWallMesh) (Utilities|Select :Index (Math|Random|RandomIntegerinRange 0 3) :Option%200 "/Game/InfiniteMatrix/Meshes/SM_Hole_01.SM_Hole_01" :Option%201 "/Game/InfiniteMatrix/Meshes/SM_Hole_02.SM_Hole_02" :Option%202 "/Game/InfiniteMatrix/Meshes/SM_Hole_03.SM_Hole_03" :Option%203 "/Game/InfiniteMatrix/Meshes/SM_Hole_04.SM_Hole_04"))
  (Transformation|AddLocalRotation (Variables|Default|GetWallMesh) (Math|Rotator|MakeRotator (Math|Random|RandomFloatinRange 0.0 3.6e+02) 0.0 0.0) false false))

(fn GenerateHealthPack
  (bind _healthpack (Variables|Default|GetHealthPack))
  (Transformation|AddLocalOffset _healthpack (Math|Vector|MakeVector (Math|Conversions|ToFloat(Integer) (Math|Random|RandomInteger 1100)) (Math|Conversions|ToFloat(Integer) (Math|Random|RandomIntegerinRange -250 250)) (Math|Conversions|ToFloat(Integer) (Math|Random|RandomIntegerinRange -250 250))) false false)
  (Math|Float|CompareFloat (Math|Random|RandomFloat) 0.2
    (:>
      (Components|DestroyComponent _healthpack))))

(fn GenerateEnemies
  (for _index (range 0 (Math|Random|RandomInteger 2))
    (bind _returnvalue (Game|SpawnActorfromClass "/Game/InfiniteMatrix/Blueprints/Enemy.Enemy_C" (Math|Conversions|ToTransform(Vector) (+ (Math|Vector|MakeVector (Math|Random|RandomFloatinRange 5e+02 2.2e+03) (Math|Random|RandomFloatinRange -3e+02 3e+02) (Math|Random|RandomFloatinRange -3e+02 3e+02)) (Transformation|GetActorLocation))) "AlwaysSpawn" 0 0))
    (Variables|/Game/InfiniteMatrix/Blueprints/Enemy.Enemy_C|SetMaster _returnvalue self)))