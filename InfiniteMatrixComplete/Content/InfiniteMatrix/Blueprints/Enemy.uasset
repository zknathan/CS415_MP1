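; Enemy actor that damages the player on contact and can be shot down by bullets for score.
; A Sphere hit on BP_Player decreases health and destroys the enemy.
; Bullet hits or overlaps share one path that raises the bullet Master's score, then destroys both bullet and enemy.
; Tick also destroys the enemy once its own Master reference is no longer valid.
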(event OnComponentHit(Sphere)
  (params (HitComponent :type Primitive%20Component%20Object%20Reference) (OtherActor :type Actor%20Object%20Reference) (OtherComp :type Primitive%20Component%20Object%20Reference) (NormalImpulse :type Vector :default "0, 0, 0") (Hit :type Hit%20Result%20Structure%20%28by%20ref%29))
  (bind _asbp_player (Utilities|Casting|CastToBP_Player OtherActor)
    (:then
      (Default|DecreaseHealth _asbp_player 5))
    (:CastFailed
      (bind _asbullet (Utilities|Casting|CastToBullet (stale OnComponentBeginOverlap(Sphere) OtherActor)))
      (Default|IncreaseScore (Variables|/Game/InfiniteMatrix/Blueprints/Bullet.Bullet_C|GetMaster _asbullet) 2)
      (Actor|DestroyActor _asbullet)))
  (Actor|DestroyActor))

(event OnComponentBeginOverlap(Sphere)
  (params (OverlappedComponent :type Primitive%20Component%20Object%20Reference) (OtherActor :type Actor%20Object%20Reference) (OtherComp :type Primitive%20Component%20Object%20Reference) (OtherBodyIndex :type Integer) (bFromSweep :type Boolean) (SweepResult :type Hit%20Result%20Structure%20%28by%20ref%29))
  (bind _asbullet (Utilities|Casting|CastToBullet OtherActor))
  (Default|IncreaseScore (Variables|/Game/InfiniteMatrix/Blueprints/Bullet.Bullet_C|GetMaster _asbullet) 2)
  (Actor|DestroyActor _asbullet)
  (Actor|DestroyActor))

(event EventBeginPlay)

(event Collision|EventActorBeginOverlap
  (params (OtherActor :type Actor%20Object%20Reference)))

(event EventTick
  (params (DeltaSeconds :type Float%20%28single-precision%29))
  (Utilities|IsValid (Variables|Default|GetMaster)
    (:Is%20Not%20Valid
      (Actor|DestroyActor))))

(fn ConstructionScript)